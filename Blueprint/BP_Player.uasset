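; BP_Player is a player pawn with movement, yaw-only look, a crosshair HUD and a prototype shooting action.
; Input axes move it along control-rotation vectors, and BeginPlay creates the HUD_Viseur widget.
; Shoot calls an event named for the server, which line-traces forward from the camera on the Visibility channel.
; A hit on another BP_Player only prints that actor's name, with no damage applied.
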(event `InputAxis|MoveFront`
  (params (AxisValue :type "Float (single-precision)"))
  ;[1 1 1] Movement
  (`self.AddMovementInput` (`KismetMathLibrary.GetForwardVector` (`self.GetControlRotation`)) AxisValue))

(event `InputAxis|MoveSide`
  (params (AxisValue :type "Float (single-precision)"))
  ;[1 1 1] Movement
  (`self.AddMovementInput` (`KismetMathLibrary.GetRightVector` (`self.GetControlRotation`)) AxisValue))

(event `InputAxis|LookSide`
  (params (AxisValue :type "Float (single-precision)"))
  ;[1 1 1] Camera
  (`self.AddControllerYawInput` AxisValue))

(event `self.ReceiveBeginPlay`
  ;[1 0.1784 0.8721] Affich. Viseur
  (bind _returnvalue (`|CreateWidget` "/Game/HUDs/HUD_Viseur.HUD_Viseur_C"))
  (bind _output_get (set `self.MonViseur` _returnvalue))
  (`UserWidget.AddToViewport` _output_get 0))

(event `InputAction|Shoot`
  (params (Key :type "Key Structure"))
  ;[1 1 1] Shoot
  (:`Pressed`
    (`self.Shoot_Serveur`)))

(event `Shoot_Serveur`
  (bind _camera (`self.Camera`))
  (bind _returnvalue (`SceneComponent.K2_GetComponentLocation` _camera))
  ;[1 1 1] Shoot
  (bind _outhit (`KismetSystemLibrary.LineTraceSingle` _returnvalue (+ _returnvalue (* (`SceneComponent.GetForwardVector` _camera) 1000)) "TraceTypeQuery1"))
  (bind (_bblockinghit _binitialoverlap _time _distance _location _impactpoint _normal _impactnormal _physmat _hitactor) (`GameplayStatics.BreakHitResult` _outhit))
  (cast `/Blueprint/BP_Player` _hitactor)
  (`KismetSystemLibrary.PrintString` (`KismetSystemLibrary.GetDisplayName` _hitactor)))

(fn `UserConstructionScript`)